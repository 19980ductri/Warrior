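; Gameplay ability that equips the hero's axe, playing an equip montage and ending when the montage finishes or is interrupted.
; On the montage's equip gameplay event, it marks the axe as the current weapon and attaches it to the right-hand socket.
; HandleEquipWeapon then applies the weapon data: linked anim layers, input mapping context, granted weapon abilities with stored spec handles, and a HUD icon update.
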(event `self.K2_ActivateAbility`
  (`AbilityTask_PlayMontageAndWait.CreatePlayMontageAndWaitProxy` "None" "/Game/Blueprint/PlayerCharacter/Montages/AM_Hero_EquipAxe.AM_Hero_EquipAxe"
    (:`then`
      (`AbilityTask_WaitGameplayEvent.WaitGameplayEvent` (struct :`TagName` "Player.Event.Equip.Axe") null
        (:`EventReceived`
          (set `PawnCombatComponent.CurrentEquippedWeaponTag` (struct :`TagName` "Player.Weapon.Axe") (`self.GetHeroCombatComponentFromActorInfo`))
          (`Actor.K2_AttachToComponent` (`PawnCombatComponent.GetCarriedWeaponByTag` (`self.GetHeroCombatComponentFromActorInfo`) (struct :`TagName` "Player.Weapon.Axe")) (`self.GetOwningComponentFromActorInfo`) "AxeRightHandSocket" "SnapToTarget" "KeepRelative" "KeepWorld" true)
          (bind _returnvalue (`HeroCombatComponent.GetHeroCarriedWeaponByTag` (`self.GetHeroCombatComponentFromActorInfo`) (struct :`TagName` "Player.Weapon.Axe")))
          (`self.HandleEquipWeapon` _returnvalue))))
    (:`OnCompleted`
      (`self.K2_EndAbility` :!label _label))
    (:`OnBlendOut`
      (goto _label))
    (:`OnInterrupted`
      (goto _label))
    (:`OnCancelled`
      (goto _label))))

(event `self.K2_OnEndAbility`
  (params (bWasCancelled :type Boolean)))

(fn `HandleEquipWeapon`
  (params (InWeapon :type "WarriorHeroWeapon Object Reference"))
  (locals (CachedHeroWeaponData :type "WarriorHeroWeaponData Structure"))
  (bind (_cachedheroweapondata_weaponanimlayertolink _cachedheroweapondata_weaponinputmappingcontext _cachedheroweapondata_defaultweaponabilities _cachedheroweapondata_weaponbasedamage _cachedheroweapondata_softweaponicon2d) (break `WarriorHeroWeaponData` (`local.CachedHeroWeaponData`)))
  (bind _cachedheroweapondata_weaponanimlayertolink_2 (break `WarriorHeroWeaponData` (`local.CachedHeroWeaponData`)))
  (bind (_cachedheroweapondata_weaponanimlayertolink_3 _cachedheroweapondata_weaponinputmappingcontext_2) (break `WarriorHeroWeaponData` (`local.CachedHeroWeaponData`)))
  (bind (_cachedheroweapondata_weaponanimlayertolink_4 _cachedheroweapondata_weaponinputmappingcontext_3 _cachedheroweapondata_defaultweaponabilities_2) (break `WarriorHeroWeaponData` (`local.CachedHeroWeaponData`)))
  (set `local.CachedHeroWeaponData` (`WarriorHeroWeapon.WeaponData` InWeapon))
  (`|ExecutionSequence`
    (:`then_0`
      (`SkeletalMeshComponent.LinkAnimClassLayers` (`self.GetOwningComponentFromActorInfo`) _cachedheroweapondata_weaponanimlayertolink_2))
    (:`then_1`
      (`EnhancedInputSubsystemInterface.AddMappingContext` (pcsubsystem `EnhancedInputLocalPlayerSubsystem` (`self.GetHeroControllerFromActorInfo`)) _cachedheroweapondata_weaponinputmappingcontext_2 0 (struct)))
    (:`then_2`
      (bind _returnvalue (`WarriorAbilitySystemComponent.GrandWeaponAbilities` (`self.GetWarriorAbilitySystemComponentFromActorInfo`) _cachedheroweapondata_defaultweaponabilities_2 1))
      (`WarriorHeroWeapon.AssignGrantedAbilitySpecHandles` (`local.InWeapon`) _returnvalue))
    (:`then_3`
      (`HeroUIComponent.OnEquippedWeaponChanged` (`WarriorHeroCharacter.HeroUIComponent` (`self.GetHeroCharacterFromActorInfo`)) _cachedheroweapondata_softweaponicon2d))))