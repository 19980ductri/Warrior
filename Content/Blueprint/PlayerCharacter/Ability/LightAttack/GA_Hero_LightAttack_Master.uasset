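; Master gameplay ability for the hero's light attack combo, stepping through mapped montages and resetting after a short idle timer.
; The JumpToFinisher tag, added before the last step, forces the finisher montage and clears on reset.
; MeleeHit events apply combo-aware weapon damage, play a hit sound cue, send HitReact and grant rage on successful hits.
; Active rage triggers WhileRageActive, an empty hook in this class.
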(event `self.K2_ActivateAbility`
  (`KismetSystemLibrary.K2_ClearAndInvalidateTimerHandle` (`self.ComboResetTimerHandle`))
  (`WarriorFunctionLibrary.BP_DoesActorHaveTag` (`self.GetHeroCharacterFromActorInfo`) (struct :`TagName` "Player.Status.JumpToFinisher")
    (:`Yes`
      (set `self.CurrentLightAttackComboCount` (`BlueprintMapLibrary.Map_Length` (`self.AttackMontagesMap`))))
    (:`No`
      _))
  (set `self.UsedLightComboCount` (`self.CurrentLightAttackComboCount`))
  (`AbilityTask_PlayMontageAndWait.CreatePlayMontageAndWaitProxy` "None" (`BlueprintMapLibrary.Map_Find` (`self.AttackMontagesMap`) (`self.CurrentLightAttackComboCount`))
    (:`then`
      (`|ExecutionSequence`
        (:`then_0`
          ; Handle DMG
          (bind (_asynctaskproxy _payload) (`AbilityTask_WaitGameplayEvent.WaitGameplayEvent` (struct :`TagName` "Shared.Event.MeleeHit") null)
            (:`EventReceived`
              (`self.HandleApplyDamage` _payload))))
        (:`then_1`
          ; Handle Combo count
          (if (== (`self.CurrentLightAttackComboCount`) (`BlueprintMapLibrary.Map_Length` (`self.AttackMontagesMap`)))
            (`self.ResetAttackComboCount`)
            (else
              (if (== (`self.CurrentLightAttackComboCount`) (- (`BlueprintMapLibrary.Map_Length` (`self.AttackMontagesMap`)) 1))
                (`WarriorFunctionLibrary.AddGameplayTagToActorIfNone` (`self.GetHeroCharacterFromActorInfo`) (struct :`TagName` "Player.Status.JumpToFinisher")))
              (`/Engine/EditorBlueprintResources/StandardMacros.IncrementInt` (`self.CurrentLightAttackComboCount`)))))
        (:`then_2`
          (`WarriorFunctionLibrary.BP_DoesActorHaveTag` (`self.GetHeroCharacterFromActorInfo`) (struct :`TagName` "Player.Status.Rage.Active")
            (:`Yes`
              (`self.WhileRageActive`))))))
    (:`OnCompleted`
      (`self.K2_EndAbility` :!label _label)
      (bind _returnvalue (`KismetSystemLibrary.K2_SetTimerDelegate` (delegate `ResetAttackComboCount`) 0.6))
      (set `self.ComboResetTimerHandle` _returnvalue))
    (:`OnBlendOut`
      (goto _label))
    (:`OnInterrupted`
      (goto _label))
    (:`OnCancelled`
      (goto _label))))

(event `WhileRageActive`)

(event `ResetAttackComboCount`
  (set `self.CurrentLightAttackComboCount` 1)
  (`WarriorFunctionLibrary.RemoveGameplayTagIfFound` (`self.GetHeroCharacterFromActorInfo`) (struct :`TagName` "Player.Status.JumpToFinisher")))

(event `self.K2_OnEndAbility`
  (params (bWasCancelled :type Boolean)))

(fn `HandleApplyDamage`
  (params (GameplayEventData :type "GameplayEventData Structure (by ref)"))
  (locals (LocalTargetActor :type "Actor Object Reference"))
  (bind _output_get (set `local.LocalTargetActor` (`.Target` (break `GameplayEventData` GameplayEventData))))
  (`self.K2_ExecuteGameplayCue` (`self.WeaponHitSoundGameplayCueTag`))
  (`self.BP_ApplyEffectSpecHandleToTarget` _output_get (`self.MakeHeroDamageEffectSpecHandle` "/Game/Shared/GameplayEffects/GE_Shared_DealDamage.GE_Shared_DealDamage_C" (`HeroCombatComponent.GetHeroCurrentEquipWeaponDamageAtLevel` (`self.GetHeroCombatComponentFromActorInfo`) (`KismetMathLibrary.Conv_IntToDouble` (`self.GetAbilityLevel`))) (struct :`TagName` "Player.SetByCaller.AttackType.Light") (`self.UsedLightComboCount`))
    (:`Successful`
      (`AbilitySystemBlueprintLibrary.SendGameplayEventToActor` (`local.LocalTargetActor`) (struct :`TagName` "Shared.Event.HitReact") (`local.GameplayEventData`))
      (`self.BP_ApplyGameplayEffectToOwner` "/Game/Blueprint/PlayerCharacter/GameplayEffect/GE_Hero_GainRage.GE_Hero_GainRage_C" (`self.GetAbilityLevel`)))))