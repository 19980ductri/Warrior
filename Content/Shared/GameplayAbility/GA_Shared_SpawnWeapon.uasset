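; Shared gameplay ability that spawns a configurable weapon for the avatar and registers it with that pawn's combat component.
; On activation it spawns the weapon class with the avatar as owner and instigator, then attaches it to the owning component at a configurable socket.
; It registers the weapon under a tag, optionally as equipped, and ends itself only when the spawn is valid.
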(event `self.K2_ActivateAbility`
  (bind _returnvalue (`self.GetAvatarActorFromActorInfo`))
  (bind _returnvalue_2 (`|SpawnActorFromClass` (`self.WeaponClassToSpawn`) (`KismetMathLibrary.MakeTransform` (0.0 0.0 0.0)) "AdjustIfPossibleButAlwaysSpawn" "MultiplyWithRoot" _returnvalue (cast `Pawn` _returnvalue :!pure true)))
  (`/Engine/EditorBlueprintResources/StandardMacros.IsValid` _returnvalue_2
    (:`Is Valid`
      (bind _output_get (set `self.SpawnedWeapon` _returnvalue_2))
      (`Actor.K2_AttachToComponent` _output_get (`self.GetOwningComponentFromActorInfo`) (`self.SocketNameToAttachTo`) "KeepRelative" "KeepRelative" "KeepRelative" true)
      (`PawnCombatComponent.RegisterSpawnedWeapon` (`self.GetPawnCombatComponentFromActorInfo`) (`self.WeaponTag`) (`self.SpawnedWeapon`) (`self.RegisterAsEquippedWeapon`))
      (`self.K2_EndAbility`))))